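; Randomly spawned absorption pickup that the player absorbs by touching it.
; One second after BeginPlay it arms its overlap check, sets its RandomSpawn state and runs its random init.
; When the player overlaps AbsBox, it passes its HP to PlayerGameInstanceSubsystem via SetAddDamage, decrements the RandomSpawner count and destroys itself.
; An unconnected chain that would attach a PlayerCube child actor to the player never runs.
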(event OnComponentBeginOverlap(absBox)
  (params (OverlappedComponent :type Primitive%20Component%20Object%20Reference) (OtherActor :type Actor%20Object%20Reference) (OtherComp :type Primitive%20Component%20Object%20Reference) (OtherBodyIndex :type Integer) (bFromSweep :type Boolean) (SweepResult :type Hit%20Result%20Structure%20%28by%20ref%29))
  ;[1 1 1] Absorption Enemy Die => PlayerAddHp
  (if (Variables|Default|GetAbsorptionSpawnCheck)
    (if (!= OtherActor self)
      (bind _asthird_person_character (Utilities|Casting|CastToThirdPersonCharacter (Game|GetPlayerCharacter 0)))
      (if (== _asthird_person_character OtherActor)
        (Class|PlayerGameInstanceSubsystem|SetAddDamage (Subsystems|GetPlayerGameInstanceSubsystem) (Variables|Default|GetAbsorptionHp))
        (bind _returnvalue (Actor|GetActorOfClass "/Game/Absorption/RandomSpawner.RandomSpawner_C"))
        (Variables|/Game/Absorption/RandomSpawner.RandomSpawner_C|SetSpawnCount _returnvalue (- (Variables|/Game/Absorption/RandomSpawner.RandomSpawner_C|GetSpawnCount _returnvalue) 1))
        (Actor|DestroyActor)))))

(event EventBeginPlay
  ;[1 1 1] Absorption Spawn Check
  (Utilities|FlowControl|Delay 1.0)
  (Variables|Default|SetAbsorptionSpawnCheck true)
  (Variables|Default|SetAbsorptionState "RandomSpawn")
  (Variables|Default|SetAbsorptionHp 1)
  (Class|Absorption|AbsorptionRandomInit))

(event EventTick
  (params (DeltaSeconds :type Float%20%28single-precision%29)))

(event EventDestroyed)

(fn ConstructionScript)