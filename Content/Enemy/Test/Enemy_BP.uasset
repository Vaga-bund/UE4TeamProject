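; Test enemy actor that can be absorbed once its HP is zero, leaving an Absorption_BP behind.
; BeginPlay caches its starting transform and spawns a MonsterPowerBP combat-power bar at the Follow component's location.
; An AbsBox overlap with another actor destroys the enemy if EnemyHp is zero.
; Destroyed then spawns Absorption_BP at the cached starting transform rather than the enemy's current one.
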(event OnComponentBeginOverlap(absBox)
  (params (OverlappedComponent :type Primitive%20Component%20Object%20Reference) (OtherActor :type Actor%20Object%20Reference) (OtherComp :type Primitive%20Component%20Object%20Reference) (OtherBodyIndex :type Integer) (bFromSweep :type Boolean) (SweepResult :type Hit%20Result%20Structure%20%28by%20ref%29))
  ;[1 1 1] ActorDestroy
  (if (!= OtherActor self)
    (if (== (Variables|Default|GetEnemyHp) 0)
      (Actor|DestroyActor))))

(event Collision|EventActorBeginOverlap
  (params (OtherActor :type Actor%20Object%20Reference)))

(event EventTick
  (params (DeltaSeconds :type Float%20%28single-precision%29)))

(event EventDestroyed
  ;[1 1 1] Enemy Destroy after spawnAbsorption
  (Game|SpawnActorfromClass "/Game/Absorption/Absorption_BP.Absorption_BP_C" (Variables|Default|GetSpawn%20Transform) "Undefined" 0 0))

(event EventBeginPlay
  ;[1 1 1] Absorption Transform
  (Variables|Default|SetSpawn%20Transform (Transformation|GetActorTransform))
  ;[1 1 1] 전투력바 소환
  (bind _returnvalue (Game|SpawnActorfromClass "/Game/UI/MonsterPowerBP.MonsterPowerBP_C" (Math|Conversions|ToTransform(Vector) (Transformation|GetWorldLocation (Variables|Default|GetFollow))) "Undefined" 0 0))
  (Variables|Default|SetpowerBar _returnvalue))

(fn ConstructionScript)