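; MonsterBP is an enemy with a power value shown on a separately spawned MonsterPowerBP bar that follows it each tick.
; Box overlap with the player saves the transform and calls Crash, while other overlaps go to AddMonster.
; The bar refreshes after a crash only if power remains, avoiding access to a destroyed bar, and through SetUIPowerCpp.
; On destruction it removes the bar and spawns an Absorption_BP at the saved transform.
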(event OnComponentBeginOverlap(Box)
  (params (OverlappedComponent :type Primitive%20Component%20Object%20Reference) (OtherActor :type Actor%20Object%20Reference) (OtherComp :type Primitive%20Component%20Object%20Reference) (OtherBodyIndex :type Integer) (bFromSweep :type Boolean) (SweepResult :type Hit%20Result%20Structure%20%28by%20ref%29))
  ;[1 1 1] 부딪쳤을 때
  (if (== OtherActor (Game|GetPlayerCharacter 0))
    ;;[1 1 1] Absorption Transform
    (Variables|Default|SetSpawn%20Transform (Transformation|GetActorTransform))
    (Class|Monster|Crash)
    (if (> (Variables|Default|GetmonsterPower) 0) ; Destroyed가 먼저 실행되어 체력바가 사라지는데, 참고할 객체가 사라져 런타임 에러가 나는 것을 방지하기 위함
      (CallFunction|UIPower))
    (else
      (Class|Monster|AddMonster OtherActor))))

(event EventBeginPlay
  ;[1 1 1] 체력바 소환
  (bind _returnvalue (Game|SpawnActorfromClass "/Game/UI/MonsterPowerBP.MonsterPowerBP_C" (Math|Conversions|ToTransform(Vector) (Transformation|GetWorldLocation (Variables|Default|GetFollow))) "Undefined" 0 0))
  (Variables|Default|SetPowerBar _returnvalue)
  (CallFunction|UIPower))

(event Collision|EventActorBeginOverlap
  (params (OtherActor :type Actor%20Object%20Reference)))

(event EventTick
  (params (DeltaSeconds :type Float%20%28single-precision%29))
  ;[1 1 1] 체력바 따라다니게 만들기
  (Default|Follow (Variables|Default|GetPowerBar) (Variables|Default|GetFollow)))

(event EventSetUIPowerCpp
  (CallFunction|UIPower))

(event EventDestroyed
  ;[1 1 1] 체력바 삭제
  (Actor|DestroyActor (Variables|Default|GetPowerBar))
  ;[1 1 1] Enemy Destroy after spawnAbsorption
  (bind _returnvalue (Game|SpawnActorfromClass "/Game/Absorption/Absorption_BP.Absorption_BP_C" (Variables|Default|GetSpawn%20Transform) "Undefined" 0 0))
  (Class|Absorption|AbsorptionInit _returnvalue))

(fn ConstructionScript)

(fn UIPower
  (Default|SetUIPower (Variables|Default|GetPowerBar) (Variables|Default|GetmonsterPower)))