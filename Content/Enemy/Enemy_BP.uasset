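; Enemy actor that resolves an HP-based clash with the player when another actor overlaps its Box component.
; The side with lower HP (player on ties) gets SetSubDamage, and its Damage value is passed to the other side's SetAddDamage.
; An HP of zero triggers EnemyDie or PlayerDie instead, checking the enemy first.
; All state lives in Enemy and Player GameInstance subsystems, and the overlap filter only excludes itself.
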(event OnComponentBeginOverlap(Box)
  (params (OverlappedComponent :type Primitive%20Component%20Object%20Reference) (OtherActor :type Actor%20Object%20Reference) (OtherComp :type Primitive%20Component%20Object%20Reference) (OtherBodyIndex :type Integer) (bFromSweep :type Boolean) (SweepResult :type Hit%20Result%20Structure%20%28by%20ref%29))
  (bind _returnvalue (Subsystems|GetEnemyGameInstanceSubsystem))
  (bind _returnvalue_2 (Subsystems|GetPlayerGameInstanceSubsystem))
  (bind _returnvalue_3 (Class|EnemyGameInstanceSubsystem|GetHp _returnvalue))
  (bind _returnvalue_4 (Class|PlayerGameInstanceSubsystem|GetHp _returnvalue_2))
  (if (!= OtherActor self)
    (if (!= _returnvalue_3 0)
      (if (!= _returnvalue_4 0)
        (if (< _returnvalue_3 _returnvalue_4)
          (Class|EnemyGameInstanceSubsystem|SetSubDamage _returnvalue)
          (Class|PlayerGameInstanceSubsystem|SetAddDamage _returnvalue_2 (Variables|/Script/UE4Project.EnemyGameInstanceSubsystem|GetDamage _returnvalue))
          (else
            (Class|PlayerGameInstanceSubsystem|SetSubDamage _returnvalue_2)
            (Class|EnemyGameInstanceSubsystem|SetAddDamage _returnvalue (Variables|/Script/UE4Project.PlayerGameInstanceSubsystem|GetDamage _returnvalue_2))))
        (else
          (Class|PlayerGameInstanceSubsystem|PlayerDie _returnvalue_2)))
      (else
        (Class|EnemyGameInstanceSubsystem|EnemyDie _returnvalue)))))

(event EventBeginPlay)

(event Collision|EventActorBeginOverlap
  (params (OtherActor :type Actor%20Object%20Reference)))

(event EventTick
  (params (DeltaSeconds :type Float%20%28single-precision%29)))

(fn ConstructionScript)